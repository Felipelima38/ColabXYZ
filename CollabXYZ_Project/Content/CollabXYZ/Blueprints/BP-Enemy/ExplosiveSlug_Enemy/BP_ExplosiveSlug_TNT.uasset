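; TNT explosive actor for the Explosive Slug enemy that deals area damage on impact.
; The first mesh hit, gated by a DoOnce, runs a zero-length multi-sphere trace for pawns at the impact point, ignoring the owner and drawing debug shapes.
; Each result receives damage credited to the owner, and the destroy call sits inside that loop, so the TNT persists if no pawn is found.
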(event `self.Mesh.OnComponentHit`
  (params (HitComponent :type "PrimitiveComponent Object Reference") (OtherActor :type "Actor Object Reference") (OtherComp :type "PrimitiveComponent Object Reference") (NormalImpulse :type "Vector Structure") (Hit :type "HitResult Structure (by ref)"))
  (bind (_bblockinghit _binitialoverlap _time _distance _location) (`GameplayStatics.BreakHitResult` Hit))
  (`/Engine/EditorBlueprintResources/StandardMacros.DoOnce` false
    (:`Completed`
      (bind _outhits (`KismetSystemLibrary.SphereTraceMultiForObjects` _location _location 150.0 (`|MakeArray` "ObjectTypeQuery3" :!type "EObjectTypeQuery Enum") false (`|MakeArray` (`self.GetOwner`)) "ForDuration"))
      (for _array_element _outhits
        (`GameplayStatics.ApplyDamage` (`.HitActor` (`GameplayStatics.BreakHitResult` _array_element)) 1.0 null (`self.GetOwner`))
        (`self.K2_DestroyActor`)))))

(fn `UserConstructionScript`)