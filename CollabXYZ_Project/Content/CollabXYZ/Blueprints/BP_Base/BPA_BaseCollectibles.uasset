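; Base collectible actor that adds coins to a Character-Base on overlap.
; A VarCTColectibles struct holds each pickup's data, including its mesh and coin increment.
; The construction script applies that mesh to the Coin component, then rebuilds the struct with the actor's own class and current mesh.
; Collision overlap waits briefly, adds the increment to the character's Coin, then destroys the actor.
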(event `self.ReceiveBeginPlay`
  ;[1 1 1] Destroy actor in 38 Sec
)

(event `self.Collision.OnComponentBeginOverlap`
  (params (OverlappedComponent :type "PrimitiveComponent Object Reference") (OtherActor :type "Actor Object Reference") (OtherComp :type "PrimitiveComponent Object Reference") (OtherBodyIndex :type Integer) (bFromSweep :type Boolean) (SweepResult :type "HitResult Structure (by ref)"))
  ;[1 1 1] increment Cion to Player and Destroy Actor
  (bind _ascharacter__base (cast `/Game/CollabXYZ/Blueprints/BP-Characters/Character-Base` OtherActor))
  (`/Engine/EditorBlueprintResources/StandardMacros.IsValid` _ascharacter__base
    (:`Is Valid`
      (`KismetSystemLibrary.Delay` 0.1)
      (set `/Game/CollabXYZ/Blueprints/BP-Characters/Character-Base.Coin` (+ (`.IncrementCoin_17_DDB6CBDA476A3D32916011AB6824C23C` (break `/Game/CollabXYZ/Blueprints/Constructs/CT_collectibles` (`self.Var_CTColectibles`))) (`/Game/CollabXYZ/Blueprints/BP-Characters/Character-Base.Coin` _ascharacter__base)) _ascharacter__base)
      (`self.K2_DestroyActor`))))

(fn `UserConstructionScript`
  (bind (_typeclass _name _incrementcoin _mesh _meshmaterial) (break `/Game/CollabXYZ/Blueprints/Constructs/CT_collectibles` (`self.Var_CTColectibles`)))
  (`StaticMeshComponent.SetStaticMesh` (`self.Coin`) _mesh)
  (set `self.Var_CTColectibles` (make `/Game/CollabXYZ/Blueprints/Constructs/CT_collectibles` (`GameplayStatics.GetObjectClass` self) _name _incrementcoin (`StaticMeshComponent.StaticMesh` (`self.Coin`)) _meshmaterial)))