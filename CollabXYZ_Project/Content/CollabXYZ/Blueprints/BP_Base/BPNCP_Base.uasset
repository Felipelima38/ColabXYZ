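; Base Blueprint for NPCs that show an interaction widget, with data suggesting a wave-linked shop selling castle and player life upgrades.
; Any overlap with the collider shows the widget, switches to UI-only input and shows the cursor.
; Ending overlap hides widget and cursor, but does not restore game input.
; The construction script applies the NPCs struct's mesh, then rebuilds that struct with the actor's own class and current mesh.
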(event `self.ReceiveBeginPlay`)

(event `self.Collider.OnComponentBeginOverlap`
  (params (OverlappedComponent :type "PrimitiveComponent Object Reference") (OtherActor :type "Actor Object Reference") (OtherComp :type "PrimitiveComponent Object Reference") (OtherBodyIndex :type Integer) (bFromSweep :type Boolean) (SweepResult :type "HitResult Structure (by ref)"))
  (bind _returnvalue (`GameplayStatics.GetPlayerController` 0))
  (`SceneComponent.SetVisibility` (`self.Widget`) true false)
  (`WidgetBlueprintLibrary.SetInputMode_UIOnlyEx` _returnvalue null "DoNotLock" true)
  (set `PlayerController.bShowMouseCursor` true _returnvalue))

(event `self.Collider.OnComponentEndOverlap`
  (params (OverlappedComponent :type "PrimitiveComponent Object Reference") (OtherActor :type "Actor Object Reference") (OtherComp :type "PrimitiveComponent Object Reference") (OtherBodyIndex :type Integer))
  (`SceneComponent.SetVisibility` (`self.Widget`) false false)
  (set `PlayerController.bShowMouseCursor` false (`GameplayStatics.GetPlayerController` 0)))

(fn `UserConstructionScript`
  (bind (_actorclass _namenpc _mesh _activedwave _itemprice _incrementlifecastle _incrementlifeplayer) (break `/Game/CollabXYZ/Blueprints/Constructs/CT_NCPs` (`self.NPCs`)))
  (`SkeletalMeshComponent.SetSkeletalMeshAsset` (`self.NPC`) _mesh)
  (set `self.NPCs` (make `/Game/CollabXYZ/Blueprints/Constructs/CT_NCPs` (`GameplayStatics.GetObjectClass` self) _namenpc (`SkeletalMeshComponent.SkeletalMeshAsset` (`self.NPC`)) _activedwave _itemprice _incrementlifecastle _incrementlifeplayer)))