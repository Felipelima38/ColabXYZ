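; Light post actor that switches its point light on or off to follow the stylized sky's light visibility flag.
; Every Tick it looks up the BP_StylizedSky actor, casts it to the Classic variant and reads SetVisibilityLights.
; After a random sub-second delay, one of two timelines drives the light intensity, staggering the change.
; The construction script applies the configurable post mesh and light color.
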(event `self.ReceiveTick`
  (params (DeltaSeconds :type "Float (single-precision)"))
  (bind _pointlight1 (`self.PointLight1`))
  (bind _returnvalue (`KismetMathLibrary.FClamp` (`KismetMathLibrary.RandomFloat`) 0.01))
  (bind _returnvalue_2 (`GameplayStatics.GetActorOfClass` "/Game/SoStylized/Environment/Sky/BP_StylizedSky.BP_StylizedSky_C"))
  (bind _asbp_stylized_sky_classic (cast `/Game/SoStylized/Environment/Sky/PRESETS/BP_StylizedSky_Classic` _returnvalue_2))
  (if (`/Game/SoStylized/Environment/Sky/BP_StylizedSky.SetVisibilityLights` _asbp_stylized_sky_classic)
    (`KismetSystemLibrary.Delay` _returnvalue)
    (bind (_direction _enable) (`Timeline|EnableLight/desable`)
      (:`Update`
        (`LightComponent.SetIntensity` _pointlight1 _enable)))
    (else
      (`KismetSystemLibrary.Delay` _returnvalue)
      (bind (_direction_2 _enable_2 _desable) (`Timeline|Timeline`)
        (:`Update`
          (`LightComponent.SetIntensity` _pointlight1 _desable))))))

(fn `UserConstructionScript`
  (`StaticMeshComponent.SetStaticMesh` (`self.Post`) (`self.Mesh`))
  (`LightComponent.SetLightColor` (`self.PointLight1`) (`self.Light Color`) true))