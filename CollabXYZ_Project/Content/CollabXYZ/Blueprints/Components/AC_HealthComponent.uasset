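; Actor component that tracks health and death state, using RepNotify variables for multiplayer.
; ApplyDamage lowers Health, clamped between zero and MaxHealth, and sets Isdead at zero, which blocks further damage.
; The OnRep functions for Health and Isdead broadcast the health-changed and died events.
; Getters expose health, death state and normalized health, the last also printing its value.
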(fn `ApplyDamage`
  (params (Damage :type "Float (double-precision)"))
  (if (`self.CanReceiveDamage`)
    (bind _output_get (set `self.Health` (`KismetMathLibrary.FClamp` (- (`self.Health`) Damage) 0.0 (`self.Max_Health`))))
    (if (<= _output_get 0.0)
      (set `self.Isdead` true))))

(fn `CanReceiveDamage`
  (returns (NewParam :type Boolean))
  (return (not (`self.Isdead`))))

(fn `GetDeathState`
  (returns (Isdead :type Boolean))
  (return (`self.Isdead`)))

(fn `GetHealth`
  (returns (Health :type "Float (double-precision)"))
  (return (`self.Health`)))

(fn `GetNormalizedHealth`
  (returns (NormalizedHeath :type "Float (double-precision)"))
  (bind _returnvalue (/ (`self.Health`) (`self.Max_Health`)))
  (`KismetSystemLibrary.PrintString` (`KismetStringLibrary.Conv_DoubleToString` _returnvalue))
  (return _returnvalue))

(fn `OnRep_Health`
  (`self.OnHealthChanged` self))

(fn `OnRep_Isdead`
  (`self.OnDied`))