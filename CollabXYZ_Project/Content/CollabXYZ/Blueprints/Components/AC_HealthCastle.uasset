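; AC_HealthCastle is an actor component that tracks a castle's health and destroyed state.
; Damage and healing apply only while the castle is not destroyed and clamp health between zero and the maximum, with zero health setting the destroyed flag.
; RepNotify functions on health and the destroyed flag fire health-change and destruction dispatchers, and getters expose raw health, normalized health and destroyed state.
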(fn `FUNC_ApplyDamageCastle`
  (params (CastleDamageValue :type "Float (double-precision)"))
  (if (`self.FUNC_CanReceiveDamage`)
    (bind _output_get (set `self.HealthCastle` (`KismetMathLibrary.FClamp` (- (`self.HealthCastle`) CastleDamageValue) 0.0 (`self.MaxHealthCastle`))))
    (if (<= _output_get 0.0)
      (set `self.DestroyedCastle` true))))

(fn `FUNC_CanReceiveDamage`
  (returns (CanReceiveDamage :type Boolean))
  (return (not (`self.DestroyedCastle`))))

(fn `FUNC_GetDestroyedCastle`
  (returns (DestroyedCastle :type Boolean))
  (return (`self.DestroyedCastle`)))

(fn `FUNC_GetNormalizedHealthCastle`
  (returns (NormalizedHeathCastle :type "Float (double-precision)"))
  (return (/ (`self.HealthCastle`) (`self.MaxHealthCastle`))))

(fn `FUNC_IncrementHealthCastle`
  (params (B :type "Float (double-precision)"))
  (locals (NewLocalVar :type "Float (double-precision)"))
  (if (`self.FUNC_CanReceiveDamage`)
    (set `self.HealthCastle` (`KismetMathLibrary.FClamp` (+ (`self.HealthCastle`) B) 0.0 (`self.MaxHealthCastle`)))))

(fn `GetHealthCastle`
  (returns (HealthCastle :type "Float (double-precision)"))
  (return (`self.HealthCastle`)))

(fn `OnRep_DestroyedCastle`
  (`self.IsDestroyedCastle`))

(fn `OnRep_HealthCastle`
  (`self.OnHealthChangeCastle` self))