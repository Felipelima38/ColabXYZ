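; Fragmented Mamona actor that bursts apart into separate pieces as soon as it spawns, then removes itself.
; On BeginPlay, a constant-falloff radial impulse from the Sphere's location flings the cell and cube components outward as a velocity change.
; A timeline drives the world scale of every piece.
; Its Update output also starts a delay that destroys the actor a few seconds later.
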(event `self.ReceiveBeginPlay`
  (bind _mamona_cell_028 (`self.Mamona_cell_028`))
  (`PrimitiveComponent.AddRadialImpulse` _mamona_cell_028 (`SceneComponent.K2_GetComponentLocation` (`self.Sphere`)) 1000.0 200.0 "RIF_Constant" true)
  (`PrimitiveComponent.AddRadialImpulse` (`self.Cube_008`) (`SceneComponent.K2_GetComponentLocation` (`self.Sphere`)) 1000.0 200.0 "RIF_Constant" true)
  (`PrimitiveComponent.AddRadialImpulse` (`self.Mamona_cell_016`) (`SceneComponent.K2_GetComponentLocation` (`self.Sphere`)) 1000.0 200.0 "RIF_Constant" true)
  (`PrimitiveComponent.AddRadialImpulse` (`self.Mamona_cell_020`) (`SceneComponent.K2_GetComponentLocation` (`self.Sphere`)) 1000.0 200.0 "RIF_Constant" true)
  (`PrimitiveComponent.AddRadialImpulse` (`self.Cube_006`) (`SceneComponent.K2_GetComponentLocation` (`self.Sphere`)) 1000.0 200.0 "RIF_Constant" true)
  (`PrimitiveComponent.AddRadialImpulse` (`self.Cube_001`) (`SceneComponent.K2_GetComponentLocation` (`self.Sphere`)) 1000.0 200.0 "RIF_Constant" true)
  (`PrimitiveComponent.AddRadialImpulse` (`self.Cube_005`) (`SceneComponent.K2_GetComponentLocation` (`self.Sphere`)) 1000.0 200.0 "RIF_Constant" true)
  (`PrimitiveComponent.AddRadialImpulse` (`self.Cube_003`) (`SceneComponent.K2_GetComponentLocation` (`self.Sphere`)) 1000.0 200.0 "RIF_Constant" true)
  (`PrimitiveComponent.AddRadialImpulse` (`self.Cube_004`) (`SceneComponent.K2_GetComponentLocation` (`self.Sphere`)) 1000.0 200.0 "RIF_Constant" true)
  (`PrimitiveComponent.AddRadialImpulse` (`self.Cube_007`) (`SceneComponent.K2_GetComponentLocation` (`self.Sphere`)) 1000.0 200.0 "RIF_Constant" true)
  (`PrimitiveComponent.AddRadialImpulse` (`self.Mamona_cell_029`) (`SceneComponent.K2_GetComponentLocation` (`self.Sphere`)) 1000.0 200.0 "RIF_Constant" true)
  (`PrimitiveComponent.AddRadialImpulse` (`self.Mamona_cell_027`) (`SceneComponent.K2_GetComponentLocation` (`self.Sphere`)) 1000.0 200.0 "RIF_Constant" true)
  (`PrimitiveComponent.AddRadialImpulse` (`self.Mamona_cell_031`) (`SceneComponent.K2_GetComponentLocation` (`self.Sphere`)) 1000.0 200.0 "RIF_Constant" true)
  (`PrimitiveComponent.AddRadialImpulse` (`self.Mamona_cell_021`) (`SceneComponent.K2_GetComponentLocation` (`self.Sphere`)) 1000.0 200.0 "RIF_Constant" true)
  (`PrimitiveComponent.AddRadialImpulse` (`self.Mamona_cell_022`) (`SceneComponent.K2_GetComponentLocation` (`self.Sphere`)) 1000.0 200.0 "RIF_Constant" true)
  (`PrimitiveComponent.AddRadialImpulse` (`self.Mamona_cell_023`) (`SceneComponent.K2_GetComponentLocation` (`self.Sphere`)) 1000.0 200.0 "RIF_Constant" true)
  (`PrimitiveComponent.AddRadialImpulse` (`self.Mamona_cell_026`) (`SceneComponent.K2_GetComponentLocation` (`self.Sphere`)) 1000.0 200.0 "RIF_Constant" true)
  (`PrimitiveComponent.AddRadialImpulse` (`self.Mamona_cell_024`) (`SceneComponent.K2_GetComponentLocation` (`self.Sphere`)) 1000.0 200.0 "RIF_Constant" true)
  (`PrimitiveComponent.AddRadialImpulse` (`self.Mamona_cell_025`) (`SceneComponent.K2_GetComponentLocation` (`self.Sphere`)) 1000.0 200.0 "RIF_Constant" true)
  (bind (_direction _newtrack_0) (`Timeline|Timeline`)
    (:`Update`
      (`SceneComponent.SetWorldScale3D` _mamona_cell_028 _newtrack_0)
      (`SceneComponent.SetWorldScale3D` (`self.Cube_008`) _newtrack_0)
      (`SceneComponent.SetWorldScale3D` (`self.Mamona_cell_016`) _newtrack_0)
      (`SceneComponent.SetWorldScale3D` (`self.Mamona_cell_020`) _newtrack_0)
      (`SceneComponent.SetWorldScale3D` (`self.Cube_001`) _newtrack_0)
      (`SceneComponent.SetWorldScale3D` (`self.Cube_006`) _newtrack_0)
      (`SceneComponent.SetWorldScale3D` (`self.Cube_005`) _newtrack_0)
      (`SceneComponent.SetWorldScale3D` (`self.Cube_003`) _newtrack_0)
      (`SceneComponent.SetWorldScale3D` (`self.Cube_004`) _newtrack_0)
      (`SceneComponent.SetWorldScale3D` (`self.Cube_007`) _newtrack_0)
      (`SceneComponent.SetWorldScale3D` (`self.Mamona_cell_029`) _newtrack_0)
      (`SceneComponent.SetWorldScale3D` (`self.Mamona_cell_027`) _newtrack_0)
      (`SceneComponent.SetWorldScale3D` (`self.Mamona_cell_031`) _newtrack_0)
      (`SceneComponent.SetWorldScale3D` (`self.Mamona_cell_021`) _newtrack_0)
      (`SceneComponent.SetWorldScale3D` (`self.Mamona_cell_022`) _newtrack_0)
      (`SceneComponent.SetWorldScale3D` (`self.Mamona_cell_023`) _newtrack_0)
      (`SceneComponent.SetWorldScale3D` (`self.Mamona_cell_026`) _newtrack_0)
      (`SceneComponent.SetWorldScale3D` (`self.Mamona_cell_024`) _newtrack_0)
      (`SceneComponent.SetWorldScale3D` (`self.Mamona_cell_025`) _newtrack_0)
      (`KismetSystemLibrary.Delay` 5.0)
      (`self.K2_DestroyActor`))))

(fn `UserConstructionScript`)