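; MamonaFragmentada is a fractured ball actor, made of ten cell pieces, that bursts apart when spawned and then removes itself.
; BeginPlay applies a constant-falloff, velocity-change radial impulse to the pieces from the Sphere component's location.
; A Timeline then drives the world scale of all pieces, and a Delay chained to its update destroys the actor about five seconds after the animation starts.
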(event `self.ReceiveBeginPlay`
  (bind _bolafracture_sphere_cell (`self.BolaFracture_Sphere_cell`))
  (`PrimitiveComponent.AddRadialImpulse` _bolafracture_sphere_cell (`SceneComponent.K2_GetComponentLocation` (`self.Sphere`)) 1000.0 1000.0 "RIF_Constant" true)
  (`PrimitiveComponent.AddRadialImpulse` (`self.BolaFracture_Sphere_cell_001`) (`SceneComponent.K2_GetComponentLocation` (`self.Sphere`)) 1000.0 1000.0 "RIF_Constant" true)
  (`PrimitiveComponent.AddRadialImpulse` (`self.BolaFracture_Sphere_cell_002`) (`SceneComponent.K2_GetComponentLocation` (`self.Sphere`)) 1000.0 1000.0 "RIF_Constant" true)
  (`PrimitiveComponent.AddRadialImpulse` (`self.BolaFracture_Sphere_cell_003`) (`SceneComponent.K2_GetComponentLocation` (`self.Sphere`)) 1000.0 1000.0 "RIF_Constant" true)
  (`PrimitiveComponent.AddRadialImpulse` (`self.BolaFracture_Sphere_cell_004`) (`SceneComponent.K2_GetComponentLocation` (`self.Sphere`)) 1000.0 1000.0 "RIF_Constant" true)
  (`PrimitiveComponent.AddRadialImpulse` (`self.BolaFracture_Sphere_cell_005`) (`SceneComponent.K2_GetComponentLocation` (`self.Sphere`)) 1000.0 1000.0 "RIF_Constant" true)
  (`PrimitiveComponent.AddRadialImpulse` (`self.BolaFracture_Sphere_cell_006`) (`SceneComponent.K2_GetComponentLocation` (`self.Sphere`)) 1000.0 1000.0 "RIF_Constant" true)
  (`PrimitiveComponent.AddRadialImpulse` (`self.BolaFracture_Sphere_cell_007`) (`SceneComponent.K2_GetComponentLocation` (`self.Sphere`)) 1000.0 1000.0 "RIF_Constant" true)
  (`PrimitiveComponent.AddRadialImpulse` (`self.BolaFracture_Sphere_cell_008`) (`SceneComponent.K2_GetComponentLocation` (`self.Sphere`)) 1000.0 1000.0 "RIF_Constant" true)
  (`PrimitiveComponent.AddRadialImpulse` (`self.BolaFracture_Sphere_cell_009`) (`SceneComponent.K2_GetComponentLocation` (`self.Sphere`)) 1000.0 1000.0 "RIF_Constant" true)
  (`KismetSystemLibrary.Delay` 0.0)
  (bind (_direction _newtrack_0) (`Timeline|Timeline`)
    (:`Update`
      (`SceneComponent.SetWorldScale3D` _bolafracture_sphere_cell _newtrack_0)
      (`SceneComponent.SetWorldScale3D` (`self.BolaFracture_Sphere_cell_001`) _newtrack_0)
      (`SceneComponent.SetWorldScale3D` (`self.BolaFracture_Sphere_cell_002`) _newtrack_0)
      (`SceneComponent.SetWorldScale3D` (`self.BolaFracture_Sphere_cell_003`) _newtrack_0)
      (`SceneComponent.SetWorldScale3D` (`self.BolaFracture_Sphere_cell_004`) _newtrack_0)
      (`SceneComponent.SetWorldScale3D` (`self.BolaFracture_Sphere_cell_005`) _newtrack_0)
      (`SceneComponent.SetWorldScale3D` (`self.BolaFracture_Sphere_cell_006`) _newtrack_0)
      (`SceneComponent.SetWorldScale3D` (`self.BolaFracture_Sphere_cell_007`) _newtrack_0)
      (`SceneComponent.SetWorldScale3D` (`self.BolaFracture_Sphere_cell_008`) _newtrack_0)
      (`SceneComponent.SetWorldScale3D` (`self.BolaFracture_Sphere_cell_009`) _newtrack_0)
      (`KismetSystemLibrary.Delay` 5.0)
      (`self.K2_DestroyActor`))))

(fn `UserConstructionScript`)