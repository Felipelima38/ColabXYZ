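; BP_PlantaCarnivoraSistema is a hologram preview of a carnivorous plant that signals whether its spot is blocked.
; Box overlaps with components or actors tagged "Colisao" set the Colidiu flag and tint the hologram red, restoring blue when an overlap ends.
; An unconnected delayed loop, which never runs, would trace downward from Sphere and hold the hologram just above the hit surface.
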(event `self.Box.OnComponentBeginOverlap`
  (params (OverlappedComponent :type "PrimitiveComponent Object Reference") (OtherActor :type "Actor Object Reference") (OtherComp :type "PrimitiveComponent Object Reference") (OtherBodyIndex :type Integer) (bFromSweep :type Boolean) (SweepResult :type "HitResult Structure (by ref)"))
  (if (or (`ActorComponent.ComponentHasTag` OtherComp "Colisao") (`self.ActorHasTag` OtherActor "Colisao"))
    (bind _returnvalue (`PrimitiveComponent.CreateDynamicMaterialInstance` (`self.Holograma Planta Carnivora`) 0 null "None"))
    (`MaterialInstanceDynamic.SetVectorParameterValue` _returnvalue "ColorOverride" (struct :`R` 0.838542 :`G` 0.087348 :`B` 0.087348 :`A` 1.0))
    (set `self.Colidiu` true)))

(event `self.Box.OnComponentEndOverlap`
  (params (OverlappedComponent :type "PrimitiveComponent Object Reference") (OtherActor :type "Actor Object Reference") (OtherComp :type "PrimitiveComponent Object Reference") (OtherBodyIndex :type Integer))
  (if (or (`ActorComponent.ComponentHasTag` OtherComp "Colisao") (`self.ActorHasTag` OtherActor "Colisao"))
    (bind _returnvalue (`PrimitiveComponent.CreateDynamicMaterialInstance` (`self.Holograma Planta Carnivora`) 0 null "None"))
    (`MaterialInstanceDynamic.SetVectorParameterValue` _returnvalue "ColorOverride" (struct :`G` 0.677171 :`B` 1.0 :`A` 1.0))
    (set `self.Colidiu` false)))

(fn `UserConstructionScript`)