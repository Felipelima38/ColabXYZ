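; An animation notify state that deals melee damage to Player-tagged pawns during its window in a montage or animation.
; Each notify tick runs a multi-sphere object trace at a configurable socket on the mesh, ignoring the owner and drawing debug spheres.
; Only the first hit is evaluated before returning; a tagged player receives base damage, with no guard against repeat damage on later ticks.
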(fn `Received_NotifyTick`
  (params (MeshComp :type "SkeletalMeshComponent Object Reference") (Animation :type "AnimSequenceBase Object Reference") (FrameDeltaTime :type "Float (single-precision)") (EventReference :type "AnimNotifyEventReference Structure (by ref)"))
  (returns (ReturnValue :type Boolean))
  (bind _returnvalue (`ActorComponent.GetOwner` MeshComp))
  (bind _returnvalue_2 (`SceneComponent.GetSocketLocation` MeshComp (`self.Socket Name`)))
  (bind _outhits (`KismetSystemLibrary.SphereTraceMultiForObjects` _returnvalue _returnvalue_2 _returnvalue_2 (`self.Radius Sphere`) (`|MakeArray` "ObjectTypeQuery3" :!type "EObjectTypeQuery Enum") false (`|MakeArray` _returnvalue) "ForDuration" true (struct :`R` 1.0 :`A` 1.0) (struct :`G` 1.0 :`A` 1.0) 1.0))
  (for _array_element _outhits
    (bind (_bblockinghit _binitialoverlap _time _distance _location _impactpoint _normal _impactnormal _physmat _hitactor) (`GameplayStatics.BreakHitResult` _array_element))
    (if (`Actor.ActorHasTag` _hitactor "Player")
      (`GameplayStatics.ApplyDamage` _hitactor (`self.Base Damage`) null _returnvalue)
      (return false)
      (else
        (return false)))))