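; Behavior Tree task that finds a player for an AI pawn to target.
; Each tick it runs a wide, zero-length sphere trace for Pawn objects at the pawn's location, ignoring itself and its parent actor.
; If the single hit is tagged Player, it stores that actor in the Target blackboard key and succeeds; otherwise it keeps running.
; Debug drawing and a name print are left in.
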(event `self.ReceiveTickAI`
  (params (OwnerController :type "AIController Object Reference") (ControlledPawn :type "Pawn Object Reference") (DeltaSeconds :type "Float (single-precision)"))
  (bind _returnvalue (`Actor.K2_GetActorLocation` ControlledPawn))
  (bind (_outhit _returnvalue_2) (`KismetSystemLibrary.SphereTraceSingleForObjects` _returnvalue _returnvalue 1500.0 (`|MakeArray` "ObjectTypeQuery3" :!type "EObjectTypeQuery Enum") false (`|MakeArray` ControlledPawn null (`Actor.GetParentActor` ControlledPawn) :!type "Actor Object Reference") "ForDuration"))
  (if _returnvalue_2
    (bind (_bblockinghit _binitialoverlap _time _distance _location _impactpoint _normal _impactnormal _physmat _hitactor) (`GameplayStatics.BreakHitResult` _outhit))
    (if (`Actor.ActorHasTag` _hitactor "Player")
      (`KismetSystemLibrary.PrintString` (`KismetSystemLibrary.GetObjectName` _hitactor))
      (`BTFunctionLibrary.SetBlackboardValueAsObject` (`self.Target`) _hitactor)
      (`self.FinishExecute` true))))