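; Gameplay player controller that ends the match when the castle is destroyed or the controlled pawn dies.
; On BeginPlay it binds to the BPA_Castle health component's destroyed event and the pawn health component's death event.
; Finish and PlayerDied share one sequence: show WB_FinishMatch, wait briefly, destroy the session through the game instance, then open Map_Menu.
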(event `self.ReceiveBeginPlay`
  ;[1 1 1] Verifica se o portão ou player esta vivo, chama eventos abaixo para voltar ao meny
  (`|ExecutionSequence`
    (:`then_0`
      (`self.FUNC_DestroyedCastle`))
    (:`then_1`
      (`self.FUNC_PlayerOnDied`))))

(event `Event Finish`
  (`self.FUNC_Widget-FinishMatch` :!label _label)
  (`KismetSystemLibrary.Delay` 2.0)
  (`self.FUNC_ReturnMenu`))

(event `Event Player Died`
  (goto _label))

(fn `FUNC_DestroyedCastle`
  (bind _returnvalue (`GameplayStatics.GetActorOfClass` "/Game/CollabXYZ/Blueprints/Actors/BPA_Castle.BPA_Castle_C"))
  (`/Engine/EditorBlueprintResources/StandardMacros.IsValid` _returnvalue
    (:`Is Valid`
      (add `/Game/CollabXYZ/Blueprints/Components/AC_HealthCastle.IsDestroyedCastle` (`/Game/CollabXYZ/Blueprints/Actors/BPA_Castle.AC_HealthCastle` _returnvalue) (`|CreateDelegate` :!event `Event Finish`)))))

(fn `FUNC_PlayerOnDied`
  (bind _healthcomponent (`/Game/CollabXYZ/Blueprints/Libery/BFL_HealthPlayer.Find Health Component` (`self.K2_GetPawn`)))
  (`/Engine/EditorBlueprintResources/StandardMacros.IsValid` _healthcomponent
    (:`Is Valid`
      (add `/Game/CollabXYZ/Blueprints/Components/AC_HealthComponent.OnDied` _healthcomponent (`|CreateDelegate` :!event `Event Player Died`)))))

(fn `FUNC_ReturnMenu`
  (bind _asgame_instance__geral (cast `/Game/CollabXYZ/Blueprints/Config-Game/Game_Instance-Geral` (`GameplayStatics.GetGameInstance`)))
  (`/Game/CollabXYZ/Blueprints/Config-Game/Game_Instance-Geral.INST_DestroySession` _asgame_instance__geral self)
  (`GameplayStatics.OpenLevel` "Map_Menu"))

(fn `FUNC_Widget-FinishMatch`
  (bind _returnvalue (`|CreateWidget` "/Game/CollabXYZ/Widgets/Widget_HUD/WB_FinishMatch.WB_FinishMatch_C" (`GameplayStatics.GetPlayerController` 0)))
  (`UserWidget.AddToViewport` _returnvalue 0))

(fn `UserConstructionScript`)