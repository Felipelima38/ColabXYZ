(event `INST_CreateSession`
  (params (PlayerController :type "PlayerController Object Reference"))
  ;[1 0.2031 0.2031] Instance Multiplayer
  ;;[1 1 1] Criar sessão multiplayer / singleplayer
  (`CreateSessionCallbackProxyAdvanced.CreateAdvancedSession` :`PlayerController` PlayerController :`PublicConnections` 5 :`PrivateConnections` 5
    (:`then`
      (`GameplayStatics.OpenLevel` "Level1" true "listen" :!label _label)
      (`KismetSystemLibrary.PrintString` "Level1"))
    (:`OnSuccess`
      (goto _label))
    (:`OnFailure`
      (`KismetSystemLibrary.PrintString` "Falha ao criar Sessão"))))

(event `INST_SearchSession`
  (params (PlayerController :type "PlayerController Object Reference"))
  ;[1 0.2031 0.2031] Instance Multiplayer
  ;;[1 1 1] Procurar sessão ativa
  (bind _results (`FindSessionsCallbackProxyAdvanced.FindSessionsAdvanced` PlayerController 2 false "AllServers" :!label _label_2)
    (:`OnSuccess`
      (for _array_element _results
        (set `self.Var_FindSession` _array_element))
      (if (not (`AdvancedSessionsLibrary.IsValidSession` (`self.Var_FindSession`)))
        (goto _label_2)))))

(event `INST_JoinSession`
  (params (PlayerController :type "PlayerController Object Reference"))
  ;[1 0.2031 0.2031] Instance Multiplayer
  ;;[1 1 1] Entrar ne sessão do jog]
  (`JoinSessionCallbackProxy.JoinSession` PlayerController (`self.Var_FindSession`)))

(event `INST_DestroySession`
  (params (PlayerController :type "PlayerController Object Reference"))
  ;[1 0.2031 0.2031] Instance Multiplayer
  ;;[1 1 1] Sair da Sessão
  (`DestroySessionCallbackProxy.DestroySession` PlayerController))