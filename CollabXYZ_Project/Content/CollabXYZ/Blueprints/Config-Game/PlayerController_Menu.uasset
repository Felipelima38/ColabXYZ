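; Player controller for the menu that serves as the entry point for multiplayer session actions.
; Its create, search, join and destroy events each cast the game instance to Game_Instance-Geral and call the matching INST session function, passing the controller itself.
; The controller holds no session logic of its own, and its Tick and construction script are empty.
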(event `self.ReceiveTick`
  (params (DeltaSeconds :type "Float (single-precision)")))

(event `PLRCTRL_Server_CriateSession`
  ;[1 1 1] PlayerController - Criar sessão
  (bind _asgame_instance (cast `/Game/CollabXYZ/Blueprints/Config-Game/Game_Instance-Geral` (`GameplayStatics.GetGameInstance`)))
  (`/Game/CollabXYZ/Blueprints/Config-Game/Game_Instance-Geral.INST_CreateSession` _asgame_instance self))

(event `PLRCTRL_Server_SearchSession`
  ;[1 1 1] PlayerController - Procurar sessão
  (bind _asgame_instance (cast `/Game/CollabXYZ/Blueprints/Config-Game/Game_Instance-Geral` (`GameplayStatics.GetGameInstance`)))
  (`/Game/CollabXYZ/Blueprints/Config-Game/Game_Instance-Geral.INST_SearchSession` _asgame_instance self))

(event `PLRCTRL_Server_JoinSession`
  ;[1 1 1] PlayerController - Entrar na sessão
  (bind _asgame_instance (cast `/Game/CollabXYZ/Blueprints/Config-Game/Game_Instance-Geral` (`GameplayStatics.GetGameInstance`)))
  (`/Game/CollabXYZ/Blueprints/Config-Game/Game_Instance-Geral.INST_JoinSession` _asgame_instance self))

(event `PLRCTRL_DestroySessiion`
  ;[1 1 1] PlayerController - sair da Sessão
  (bind _asgame_instance (cast `/Game/CollabXYZ/Blueprints/Config-Game/Game_Instance-Geral` (`GameplayStatics.GetGameInstance`)))
  (`/Game/CollabXYZ/Blueprints/Config-Game/Game_Instance-Geral.INST_DestroySession` _asgame_instance self))

(fn `UserConstructionScript`)