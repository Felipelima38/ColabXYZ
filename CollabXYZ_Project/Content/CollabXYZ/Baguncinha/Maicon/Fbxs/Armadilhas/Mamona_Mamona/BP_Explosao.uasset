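; BP_Explosao is a timed exploding trap actor built on a Geometry Collection.
; Three seconds after BeginPlay it pushes the collection with a radial velocity-change impulse, then briefly afterwards plays a fire-bomb particle effect and a camera shutter sound.
; The SpawnSystemAtLocation call shows no system template.
; The sphere overlap only prints a debug string, and the other impulse and collision-damage nodes are unconnected.
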(event `self.ReceiveBeginPlay`
  (bind _returnvalue (`self.K2_GetActorLocation`))
  (`KismetSystemLibrary.Delay` 3.0)
  (`PrimitiveComponent.AddRadialImpulse` (`self.GeometryCollectionComponent`) (`self.K2_GetActorLocation`) 400.0 255.0 "RIF_Constant" true)
  (`KismetSystemLibrary.Delay` 0.4)
  (`GameplayStatics.SpawnEmitterAtLocation` "/Game/InfinityBladeEffects/Effects/FX_Monsters/FX_Monster_Gruntling/Bomber/P_FireBombExplosion.P_FireBombExplosion" (`SceneComponent.K2_GetComponentLocation` (`self.GeometryCollectionComponent`)))
  (`NiagaraFunctionLibrary.SpawnSystemAtLocation` null _returnvalue)
  (`GameplayStatics.PlaySoundAtLocation` "/Engine/VREditor/Sounds/UI/Camera_Shutter.Camera_Shutter" _returnvalue (struct) 2.0 1.0 0.0 null null null null))

(event `self.Sphere.OnComponentBeginOverlap`
  (params (OverlappedComponent :type "PrimitiveComponent Object Reference") (OtherActor :type "Actor Object Reference") (OtherComp :type "PrimitiveComponent Object Reference") (OtherBodyIndex :type Integer) (bFromSweep :type Boolean) (SweepResult :type "HitResult Structure (by ref)"))
  (`KismetSystemLibrary.PrintString` "Hello"))

(fn `UserConstructionScript`)